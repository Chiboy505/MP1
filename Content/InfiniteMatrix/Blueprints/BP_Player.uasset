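; Player pawn that flies forward automatically along world X while the player steers it vertically and horizontally.
; Tick applies a swept ForwardSpeed offset until IsDead is set, a flag that this graph only reads.
; MoveUp and MoveRight add movement input scaled by the same ForwardSpeed, then immediately consume it as a swept, delta-time-scaled local offset.
; Steering does not check IsDead.
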(event `self.ReceiveBeginPlay`)

(event `self.ReceiveTick`
  (params (DeltaSeconds :type "Float (single-precision)"))
  (if (not (`self.IsDead`))
    (`self.K2_AddActorWorldOffset` (`KismetMathLibrary.MakeVector` (* DeltaSeconds (`self.ForwardSpeed`))) true)))

(event `InputAxis|MoveUp`
  (params (AxisValue :type "Float (single-precision)"))
  ;[1 1 1] Horizontal and vertical movement
  (`self.AddMovementInput` (`self.GetActorUpVector`) (* AxisValue (`self.ForwardSpeed`)))
  (bind _returnvalue (`self.ConsumeMovementInputVector` :!label _label))
  (`self.K2_AddActorLocalOffset` (* _returnvalue (`GameplayStatics.GetWorldDeltaSeconds`)) true))

(event `InputAxis|MoveRight`
  (params (AxisValue :type "Float (single-precision)"))
  ;[1 1 1] Horizontal and vertical movement
  (`self.AddMovementInput` (`self.GetActorRightVector`) (* AxisValue (`self.ForwardSpeed`)))
  (goto _label))

(fn `UserConstructionScript`)